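; Player pawn that provides an orbit camera and stepped throttle control, and creates the game HUD.
; On BeginPlay it has the first player controller possess it, enables input and adds the HUD widget to the viewport.
; Frame-time-scaled view axes rotate the controller and zoom the spring arm within limits.
; Throttle presses step a clamped value, which nothing here applies to movement, as Thrust and Tick are empty.
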(event `self.ReceiveActorBeginOverlap`
  (params (OtherActor :type "Actor Object Reference")))

(event `self.ReceiveBeginPlay`
  (bind _returnvalue (`GameplayStatics.GetPlayerController` 0))
  ;[1 1 1] Enable control keys
  (`Controller.Possess` _returnvalue self)
  (`self.EnableInput` _returnvalue)
  (bind _returnvalue_2 (`|CreateWidget` "/Game/UI/GameHUD.GameHUD_C"))
  (bind _output_get (set `self.HUD Reference` _returnvalue_2))
  (`UserWidget.AddToViewport` _output_get 0))

(event `InputAxis|ViewRotateY`
  (params (AxisValue :type "Float (single-precision)"))
  (`self.AddControllerPitchInput` (* AxisValue (`self.ViewRotation_Vspeed`) (`GameplayStatics.GetWorldDeltaSeconds`))))

(event `InputAxis|ViewRotateX`
  (params (AxisValue :type "Float (single-precision)"))
  (`self.AddControllerYawInput` (* (`GameplayStatics.GetWorldDeltaSeconds`) AxisValue (`self.ViewRotation_Hspeed`))))

(event `InputAxis|ViewZoom`
  (params (AxisValue :type "Float (single-precision)"))
  (bind _springarm (`self.SpringArm`))
  (set `SpringArmComponent.TargetArmLength` (`KismetMathLibrary.FClamp` (- (`SpringArmComponent.TargetArmLength` _springarm) (* (`GameplayStatics.GetWorldDeltaSeconds`) AxisValue (`self.ViewRotation_Zspeed`))) (`self.Zoom Minimum`) (`self.Zoom Maximum`)) _springarm))

(event `InputAction|ThrottleIncrease`
  (params (Key :type "Key Structure" :default "AnyKey"))
  (:`Pressed`
    (set `self.Throttle` (`KismetMathLibrary.FClamp` (+ (`self.Throttle`) (`self.Throttle Step`)) (`self.Throttle Minimum`) (`self.Throttle Maximum`)))))

(event `InputAction|ThrottleDecrease`
  (params (Key :type "Key Structure" :default "AnyKey"))
  (:`Pressed`
    (set `self.Throttle` (`KismetMathLibrary.FClamp` (- (`self.Throttle`) (`self.Throttle Step`)) (`self.Throttle Minimum`) (`self.Throttle Maximum`)))))

(event `InputAxis|Thrust`
  (params (AxisValue :type "Float (single-precision)")))

(event `self.ReceiveTick`
  (params (DeltaSeconds :type "Float (single-precision)")))

(fn `UserConstructionScript`)